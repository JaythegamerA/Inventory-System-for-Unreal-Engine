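; Grid inventory component that stores items spanning multiple tiles in a flattened Columns by Rows array.
; TryAddItem scans for the first top-left slot where the item's footprint is in bounds and empty, rotating the item to retry if none fits.
; Items fill every covered cell; GetAllItem maps each unique item to its top-left tile.
; Adding or removing sets a dirty flag, which Tick turns into an inventory update call.
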(event `self.ReceiveBeginPlay`
  (`KismetArrayLibrary.Array_Resize` (`self.Items`) (* (`self.Columns`) (`self.Rows`))))

(event `self.ReceiveTick`
  (params (DeltaSeconds :type "Float (single-precision)"))
  (if (`self.IsDirty`)
    (set `self.IsDirty` false)
    (`self.OnInventoryUpdate`)))

(fn `AddItem`
  (params (ItemObject :type "/Game/Inventory/Items/ItemsBlueprints/BP_ItemObject Object Reference") (TopLeft :type Integer))
  (bind _tile (`self.EachIndex` ItemObject TopLeft)
    (:`LoopBody`
      (`KismetArrayLibrary.Array_Set` (`self.Items`) (`self.TileToIndex` _tile) (`local.ItemObject`)))
    (:`Completed`
      (set `self.IsDirty` true))))

(fn `GetAllItem`
  (returns (AllItems :type "Map of /Game/Inventory/Items/ItemsBlueprints/BP_ItemObject Object Reference to /Game/Inventory/InventoryBlueprints/Tile Structure"))
  (locals (`AllItems(Local)` :type "Map of /Game/Inventory/Items/ItemsBlueprints/BP_ItemObject Object Reference to /Game/Inventory/InventoryBlueprints/Tile Structure") (`CurrentItem(Local)` :type "/Game/Inventory/Items/ItemsBlueprints/BP_ItemObject Object Reference"))
  (for (_array_element _array_index) (`self.Items`)
    (bind _output_get (set `local.CurrentItem(Local)` _array_element))
    (`/Engine/EditorBlueprintResources/StandardMacros.IsValid` _output_get
      (:`Is Valid`
        (if (not (`BlueprintMapLibrary.Map_Contains` (`local.AllItems(Local)`) _array_element))
          (`BlueprintMapLibrary.Map_Add` (`local.AllItems(Local)`) (`local.CurrentItem(Local)`) (`self.IndexToTile` _array_index))))))
  (return (`local.AllItems(Local)`)))

(fn `GetItemIndex`
  (params (Index :type Integer))
  (returns (Valid :type Boolean) (ItemObject :type "/Game/Inventory/Items/ItemsBlueprints/BP_ItemObject Object Reference"))
  (if (`KismetArrayLibrary.Array_IsValidIndex` (`self.Items`) Index)
    (return true (`|GetArrayItem` (`self.Items`) (`local.Index`)))
    (else
      (return false null))))

(fn `IndexToTile`
  (params (Idex :type Integer))
  (returns (Tile :type "/Game/Inventory/InventoryBlueprints/Tile Structure"))
  (return (make `/Game/Inventory/InventoryBlueprints/Tile` (mod Idex (`self.Columns`)) (/ Idex (`self.Columns`)))))

(fn `RemoveItem`
  (params (ItemObject :type "/Game/Inventory/Items/ItemsBlueprints/BP_ItemObject Object Reference"))
  (bind _items (`self.Items`))
  (`/Engine/EditorBlueprintResources/StandardMacros.IsValid` ItemObject
    (:`Is Valid`
      (for (_array_element _array_index) _items
        (if (== _array_element (`local.ItemObject`))
          (`KismetArrayLibrary.Array_Set` _items _array_index)
          (set `self.IsDirty` true))))))

(fn `RoomAvailble`
  (params (ItemObject :type "/Game/Inventory/Items/ItemsBlueprints/BP_ItemObject Object Reference") (TopLeft :type Integer))
  (returns (Results :type Boolean))
  (`|ExecutionSequence`
    (:`then_0`
      (bind _tile (`self.EachIndex` (`local.ItemObject`) (`local.TopLeft`))
        (:`LoopBody`
          (`self.TileValid` _tile
            (:`true`
              (bind (_valid _itemobject) (`self.GetItemIndex` (`self.TileToIndex` _tile)))
              (if _valid
                (if (`KismetSystemLibrary.IsValid` _itemobject)
                  (return false))
                (else
                  (return false))))
            (:`false`
              (return false))))))
    (:`then_1`
      (return true))))

(fn `TileToIndex`
  (params (Tile :type "/Game/Inventory/InventoryBlueprints/Tile Structure"))
  (returns (Index :type Integer))
  (bind (_x _y) (break `/Game/Inventory/InventoryBlueprints/Tile` Tile))
  (return (+ _x (* _y (`self.Columns`)))))

(fn `TryAddItem`
  (params (`Item Object` :type "/Game/Inventory/Items/ItemsBlueprints/BP_ItemObject Object Reference"))
  (returns (Added :type Boolean))
  (`/Engine/EditorBlueprintResources/StandardMacros.IsValid` `Item Object`
    (:`Is Valid`
      (for (_ _array_index) (`self.Items`) :!label _label
        (bind _results (`self.RoomAvailble` (`local.Item Object`) _array_index))
        (if _results
          (`self.AddItem` (`local.Item Object`) _array_index)
          (return true)))
      (`|ExecutionSequence`
        (:`then_0`
          (`/Engine/EditorBlueprintResources/StandardMacros.DoOnce` false
            (:`Completed`
              (`/Game/Inventory/Items/ItemsBlueprints/BP_ItemObject.Rotate` (`local.Item Object`))
              (goto _label))))))))